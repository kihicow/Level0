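; Input-driven actor, apparently a WASD-plus-Shift check, that sets physics simulation on its static mesh from movement and Sprint state.
; It enables player input at BeginPlay, and both move axes share one axis-value check that sets MovePressed.
; A Sprint press, gated by another axis-value comparison, sets SprintPressed, applies both flags' AND to SetSimulatePhysics, then disables input even if MovePressed is false.
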(event EventBeginPlay
  (Input|EnableInput (Game|GetPlayerController 0)))

(event Collision|EventActorBeginOverlap
  (params (OtherActor :type Actor%20Object%20Reference)))

(event EventTick
  (params (DeltaSeconds :type Float%20%28single-precision%29)))

(event Input|ActionEvents|InputActionSprint
  (params (Key :type Key%20Structure))
  (:Pressed
    (if (!= (stale Input|AxisEvents|InputAxisMoveForward AxisValue) (stale Input|AxisEvents|InputAxisMoveRight AxisValue))
      (bind _output_get (Variables|Default|SetSprintPressed true))
      (Physics|SetSimulatePhysics (Variables|Default|GetStaticMesh) (and _output_get (stale Input|AxisEvents|InputAxisMoveForward _output_get)))
      (Input|DisableInput (Game|GetPlayerController 0)))))

(event Input|AxisEvents|InputAxisMoveForward
  (params (AxisValue :type Float%20%28single-precision%29))
  (if (!= AxisValue (stale Input|AxisEvents|InputAxisMoveRight AxisValue))
    (bind _output_get (Variables|Default|SetMovePressed true))))

(event Input|AxisEvents|InputAxisMoveRight
  (params (AxisValue :type Float%20%28single-precision%29))
  (if (!= (stale Input|AxisEvents|InputAxisMoveForward AxisValue) AxisValue)
    (bind _output_get (Variables|Default|SetMovePressed true))))

(fn ConstructionScript)