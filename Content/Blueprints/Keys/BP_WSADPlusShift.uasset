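; Key prop actor for WSAD plus Shift that turns on physics simulation on its static mesh once both move and sprint inputs are flagged.
; It enables player input on BeginPlay, and MoveForward, MoveRight and Sprint handlers set the two flags.
; Tick applies their AND to SetSimulatePhysics every frame.
; Each handler compares AxisValue with itself, so the flags normally never get set as written.
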(event EventBeginPlay
  (bind _returnvalue (Game|GetPlayerController 0))
  (Input|EnableInput _returnvalue)
  (if (Variables|Default|GetMoveTapped)
    (Input|DisableInput _returnvalue)))

(event Collision|EventActorBeginOverlap
  (params (OtherActor :type Actor%20Object%20Reference)))

(event EventTick
  (params (DeltaSeconds :type Float%20%28single-precision%29))
  (Physics|SetSimulatePhysics (Variables|Default|GetStaticMesh) (and (Variables|Default|GetMoveTapped) (Variables|Default|GetShiftTapped))))

(event Input|ActionEvents|InputActionSprint
  (params (Key :type Key%20Structure :default "None"))
  (:Pressed
    (if (!= (stale Input|AxisEvents|InputAxisMoveForward AxisValue) (stale Input|AxisEvents|InputAxisMoveRight AxisValue))
      (Variables|Default|SetShiftTapped true))))

(event Input|AxisEvents|InputAxisMoveForward
  (params (AxisValue :type Float%20%28single-precision%29))
  (if (!= AxisValue (stale Input|AxisEvents|InputAxisMoveRight AxisValue))
    (Variables|Default|SetMoveTapped true)))

(event Input|AxisEvents|InputAxisMoveRight
  (params (AxisValue :type Float%20%28single-precision%29))
  (if (!= (stale Input|AxisEvents|InputAxisMoveForward AxisValue) AxisValue)
    (Variables|Default|SetMoveTapped true)))

(fn ConstructionScript)